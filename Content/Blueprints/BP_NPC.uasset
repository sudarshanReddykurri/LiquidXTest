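; BP_NPC is an NPC Blueprint that displays its dialogue on screen through a WBP_Dialogue widget.
; Talk defers to the parent class, while DialoguesText lazily creates the widget for player 0 and sets its text.
; NoDialoguesLeft resets TalkIndex, then removes and clears the widget reference.
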(event `self.ReceiveBeginPlay`)

(event `DIalogueInterface.Talk`
  (`parent.Talk`))

(event `self.DialoguesText`
  (params (dialogueText :type String))
  (`/Engine/EditorBlueprintResources/StandardMacros.IsValid` (`self.UI`)
    (:`Is Valid`
      _)
    (:`Is Not Valid`
      (bind _returnvalue (`|CreateWidget` "/Game/Widgets/WBP_Dialogue.WBP_Dialogue_C" (`GameplayStatics.GetPlayerController` 0)))
      (bind _output_get (set `self.UI` _returnvalue))
      (`UserWidget.AddToViewport` _output_get 0)))
  (`TextBlock.SetText` (`/Game/Widgets/WBP_Dialogue.DialougeText` (`self.UI`)) (`KismetTextLibrary.Conv_StringToText` dialogueText)))

(event `self.NoDialoguesLeft`
  (bind _ui (`self.UI`))
  (set `self.talkIndex` 0)
  (`/Engine/EditorBlueprintResources/StandardMacros.IsValid` _ui
    (:`Is Valid`
      (`Widget.RemoveFromParent` _ui)
      (set `self.UI` null))))

(fn `UserConstructionScript`)